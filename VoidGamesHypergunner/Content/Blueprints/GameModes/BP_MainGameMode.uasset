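; Main game mode that sets up a two-player local multiplayer session when play begins.
; It gathers the PlayerStart actors and spawns a BP_C_PlayerCharacter at each of the first two.
; The existing player controller possesses the first character, while a newly created local player's controller possesses the second.
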(event `self.ReceiveBeginPlay`
  (bind _outactors (`GameplayStatics.GetAllActorsOfClass` "/Script/Engine.PlayerStart"))
  (for _index (range 2)
    (if (> _index 0)
      (bind _returnvalue (`GameplayStatics.CreatePlayer` -1))
      (bind _returnvalue_2 (`self.GetTransform` (`|GetArrayItem` _outactors _index)))
      (bind _returnvalue_3 (`|SpawnActorFromClass` "/Game/Blueprints/Characters/BP_C_PlayerCharacter.BP_C_PlayerCharacter_C" _returnvalue_2 "Undefined" "MultiplyWithRoot" null null))
      (`Controller.Possess` _returnvalue _returnvalue_3)
      (else
        (bind _returnvalue_4 (`|SpawnActorFromClass` "/Game/Blueprints/Characters/BP_C_PlayerCharacter.BP_C_PlayerCharacter_C" _returnvalue_2 "Undefined" "MultiplyWithRoot" null null))
        (`Controller.Possess` (`GameplayStatics.GetPlayerController` 0) _returnvalue_4)))))

(fn `UserConstructionScript`)