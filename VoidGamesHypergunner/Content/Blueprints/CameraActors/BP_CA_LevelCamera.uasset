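; Shared level camera actor that frames two player characters, following their midpoint and zooming with their horizontal separation.
; On BeginPlay it stores its placed location as an offset, waits a tick, then enables ticking only if both players are valid.
; Each tick it eases toward the offset midpoint in X and Z, shifting Y by their X distance times a zoom factor.
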(event `self.ReceiveBeginPlay`
  (`self.SetActorTickEnabled` false)
  (`self.SaveInitialWorldLocation` self)
  (`KismetSystemLibrary.DelayUntilNextTick`)
  (bind _bareplayerreferencesvalid (`self.SavePlayerReferences` self))
  (`self.SetActorTickEnabled` _bareplayerreferencesvalid))

(event `self.ReceiveTick`
  (params (DeltaSeconds :type "Float (single-precision)"))
  (`self.SavePlayerCurrentLocations` self)
  (bind _newlocation (`self.CalculateNewTickLocation` self DeltaSeconds))
  (`self.K2_SetActorLocation` _newlocation))

(fn `CalculateNewTickLocation`
  (params (DeltaTime :type "Float (single-precision) (by ref)"))
  (returns (NewLocation :type "Vector Structure"))
  (bind _defaultworldlocation (`self.DefaultWorldLocation`))
  (bind _returnvalue_x (`KismetMathLibrary.BreakVector` (`KismetMathLibrary.Vector_GetAbs` (- (`self.Player1WorldLocation`) (`self.Player2WorldLocation`)))))
  (bind (_returnvalue_x_2 _returnvalue_y _returnvalue_z) (`KismetMathLibrary.BreakVector` (+ (/ (+ (`self.Player1WorldLocation`) (`self.Player2WorldLocation`)) 2.0) _defaultworldlocation)))
  (return (`KismetMathLibrary.VInterpTo` (`self.K2_GetActorLocation` self) (`KismetMathLibrary.MakeVector` _returnvalue_x_2 (+ (.y _defaultworldlocation) (* _returnvalue_x (`self.ZoomFactor`))) _returnvalue_z) DeltaTime (`self.CameraSmoothingSpeed`))))

(fn `SaveInitialWorldLocation`
  (set `self.DefaultWorldLocation` (`self.K2_GetActorLocation` self)))

(fn `SavePlayerCurrentLocations`
  (set `self.Player1WorldLocation` (`self.K2_GetActorLocation` (`self.PlayerCharacter1Reference`)))
  (set `self.Player2WorldLocation` (`self.K2_GetActorLocation` (`self.PlayerCharacter2Reference`))))

(fn `SavePlayerReferences`
  (returns (bArePlayerReferencesValid :type Boolean))
  (bind _returnvalue (`GameplayStatics.GetPlayerCharacter` 1))
  (bind _returnvalue_2 (`GameplayStatics.GetPlayerCharacter` 0))
  (bind _returnvalue_3 (`KismetSystemLibrary.IsValid` _returnvalue))
  (bind _returnvalue_4 (`KismetSystemLibrary.IsValid` _returnvalue_2))
  (if _returnvalue_4
    (set `self.PlayerCharacter1Reference` _returnvalue_2)
    (if _returnvalue_3
      (set `self.PlayerCharacter2Reference` _returnvalue)
      (return (and _returnvalue_4 _returnvalue_3)))))

(fn `UserConstructionScript`)