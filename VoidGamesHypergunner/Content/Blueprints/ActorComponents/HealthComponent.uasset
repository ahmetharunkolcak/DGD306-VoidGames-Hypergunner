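; Actor component that stores an actor's current and maximum health and exposes getters for both.
; Initialize sets the maximum and fills current health to it.
; UpdateHealth routes an amount to either current or maximum health, with a flag choosing add or subtract.
; Current health stays clamped between zero and the maximum, which never drops below one and re-clamps current health whenever it changes.
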(fn `GetCurrentHealth`
  (returns (CurrentHealth :type "Float (double-precision)"))
  (return (`self.CurrentHealth`)))

(fn `GetMaximumHealth`
  (returns (MaxHealth :type "Float (double-precision)"))
  (return (`self.MaximumHealth`)))

(fn `Initialize`
  (params (MaxHealth :type "Float (double-precision)"))
  (bind _output_get (set `self.MaximumHealth` MaxHealth))
  (set `self.CurrentHealth` _output_get)
  (return))

(fn `UpdateCurrentHealth`
  (params (Damage :type "Float (double-precision) (by ref)") (IsPositive :type "Boolean (by ref)"))
  (bind _maximumhealth (`self.MaximumHealth`))
  (bind _currenthealth (`self.CurrentHealth`))
  (if IsPositive
    (set `self.CurrentHealth` (`KismetMathLibrary.FClamp` (+ _currenthealth Damage) 0.0 _maximumhealth))
    (else
      (set `self.CurrentHealth` (`KismetMathLibrary.FClamp` (- _currenthealth Damage) 0.0 _maximumhealth))))
  (return))

(fn `UpdateHealth`
  (params (Damage :type "Float (double-precision)") (IsCurrentHealth :type Boolean) (IsPositive :type Boolean))
  (if IsCurrentHealth
    (`self.UpdateCurrentHealth` Damage IsPositive)
    (else
      (`self.UpdateMaximumHealth` Damage IsPositive)))
  (return))

(fn `UpdateMaximumHealth`
  (params (Damage :type "Float (double-precision) (by ref)") (IsPositive :type "Boolean (by ref)"))
  (bind _maximumhealth (`self.MaximumHealth`))
  (if IsPositive
    (set `self.MaximumHealth` (`KismetMathLibrary.FMax` 1.0 (+ _maximumhealth Damage)))
    (else
      (set `self.MaximumHealth` (`KismetMathLibrary.FMax` 1.0 (- _maximumhealth Damage)))))
  (set `self.CurrentHealth` (`KismetMathLibrary.FClamp` (`self.CurrentHealth`) 0.0 (`self.MaximumHealth`)))
  (return))